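; BP_MbRPlayerState is a player state Blueprint that appears to be a test for passing string messages between events.
; BeginPlay enables input from player controller 0.
; Server and ServerJ each set StringLmao to a fixed word and pass it to All or AllJ, which print it; the names suggest server-to-all RPCs.
; The chains that would call Server and ServerJ are unconnected, so nothing here triggers them.
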(event `self.ReceiveBeginPlay`
  (`self.EnableInput` (`GameplayStatics.GetPlayerController` 0)))

(event `Key|L`
  (params (Key :type "Key Structure")))

(event `Key|J`
  (params (Key :type "Key Structure")))

(event `ServerJ`
  (bind _output_get (set `self.StringLmao` "LMAO"))
  (`self.AllJ` _output_get))

(event `Server`
  (bind _output_get (set `self.StringLmao` "LOL"))
  (`self.All` _output_get))

(event `All`
  (params (NewParam :type String))
  (`KismetSystemLibrary.PrintString` NewParam))

(event `AllJ`
  (params (NewParam :type String))
  (`KismetSystemLibrary.PrintString` NewParam))

(fn `UserConstructionScript`)