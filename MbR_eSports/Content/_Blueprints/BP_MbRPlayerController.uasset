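; BP_MbRPlayerController is a player controller holding an unfinished relay for multiplayer text chat.
; SendMessageToServer forwards text to SendMessageToClients, which passes it to a valid ChatWidget's OnChatMessageTypedToAll.
; ReplicateOnServer stores a given widget in ChatWidget, while the OnRep function is empty.
; BeginPlay and CreateAndAddChatWidget are empty, as the widget creation, viewport and test "Hello" logic is disconnected and never runs.
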(event `CreateAndAddChatWidget`)

(event `self.ReceiveBeginPlay`)

(event `ReplicateOnServer`
  (params (NewParam :type "/Game/_Blueprints/ChatSystem/BP_ChatWidget Object Reference"))
  (set `self.chat_Widget` NewParam))

(event `Key|L`
  (params (Key :type "Key Structure")))

(event `SendMessageToServer`
  (params (NewParam :type String))
  (`self.SendMessageToClients` NewParam))

(event `SendMessageToClients`
  (params (NewParam :type String))
  (bind _chat_widget (`self.chat_Widget`))
  (if (`KismetSystemLibrary.IsValid` _chat_widget)
    (`ChatWidget.OnChatMessageTypedToAll` _chat_widget NewParam)))

(fn `OnRep_chat_Widget`)

(fn `UserConstructionScript`)